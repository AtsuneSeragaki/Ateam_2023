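; BP_Bom is a thrown bomb projectile that explodes on impact.
; On BeginPlay it finds the FirstPersonCharacter and sets its projectile movement max speed from that character's ThrowPower.
; A mesh hit spawns an explosion emitter, sets the CollisionDetection flag and gives the actor a very short remaining lifespan.
; The Ball component also sets that flag when it begins overlapping a Test actor, without exploding.
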(event `self.StaticMeshComponent.OnComponentHit`
  (params (HitComponent :type "PrimitiveComponent Object Reference") (OtherActor :type "Actor Object Reference") (OtherComp :type "PrimitiveComponent Object Reference") (NormalImpulse :type "Vector Structure") (Hit :type "HitResult Structure (by ref)"))
  (`GameplayStatics.SpawnEmitterAtLocation` "/Game/StarterContent/Particles/P_Explosion.P_Explosion" (`self.K2_GetActorLocation`))
  (set `self.collision detection` true)
  (`self.SetLifeSpan` 0.1))

(event `self.ball.OnComponentBeginOverlap`
  (params (OverlappedComponent :type "PrimitiveComponent Object Reference") (OtherActor :type "Actor Object Reference") (OtherComp :type "PrimitiveComponent Object Reference") (OtherBodyIndex :type Integer) (bFromSweep :type Boolean) (SweepResult :type "HitResult Structure (by ref)"))
  (cast `/Game/Test/Test` OtherActor)
  (set `self.collision detection` true))

(event `self.ReceiveBeginPlay`
  (bind _returnvalue (`GameplayStatics.GetActorOfClass` "/Game/FirstPersonBP/Blueprints/FirstPersonCharacter.FirstPersonCharacter_C"))
  (set `self.First` _returnvalue)
  (set `ProjectileMovementComponent.MaxSpeed` (`/Game/FirstPersonBP/Blueprints/FirstPersonCharacter.ThrowPower` (`self.First`)) (`self.ProjectileMovement`)))

(fn `UserConstructionScript`)