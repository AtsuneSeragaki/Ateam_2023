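; Damage actor in the Bom folder that hurts actors of class Test when its Ball sphere is hit.
; On BeginPlay it scales the sphere radius and damage by the player TestCharacter's RangeLevel and DamageLevel.
; Hits pass a DoOnce that resets only after damage is applied, so a hit on another class leaves it closed.
; Radial impulse, delayed destroy and tiered upgrade logic remain as unconnected nodes.
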(event `self.ReceiveBeginPlay`
  (bind _ball (`self.ball`))
  (bind _astest_character (cast `/Game/FirstPersonBP/Blueprints/TestCharacter` (`GameplayStatics.GetPlayerCharacter` 0)))
  (`SphereComponent.SetSphereRadius` _ball (* (`/Game/FirstPersonBP/Blueprints/TestCharacter.range_level` _astest_character) (`SphereComponent.SphereRadius` _ball)) true)
  (set `self.damage` (* (`/Game/FirstPersonBP/Blueprints/TestCharacter.Damage_Level` _astest_character) (`self.damage`))))

(event `self.ball.OnComponentHit`
  (params (HitComponent :type "PrimitiveComponent Object Reference") (OtherActor :type "Actor Object Reference") (OtherComp :type "PrimitiveComponent Object Reference") (NormalImpulse :type "Vector Structure") (Hit :type "HitResult Structure (by ref)"))
  (set `self.Other Actor` OtherActor)
  (`/Engine/EditorBlueprintResources/StandardMacros.DoOnce` false :!label _label
    (:`Completed`
      (if (== (`GameplayStatics.GetObjectClass` (`self.Other Actor`)) "/Game/Geometry/Meshes/Test.Test_C")
        (`GameplayStatics.ApplyDamage` (`self.Other Actor`) (`self.damage`))
        (`self.enddamage`)))))

(event `enddamage`
  (goto _label :!via `Reset`))

(fn `UserConstructionScript`)